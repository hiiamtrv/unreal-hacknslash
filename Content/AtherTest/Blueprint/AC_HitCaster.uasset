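; Actor component that detects melee weapon hits on pawns while casting is enabled through EnableCast and DisableCast.
; Each tick it box-traces between the weapon tip and base sockets on the owner's skeletal mesh.
; Each actor is handled once per cast via HitActors, which clears while casting is off.
; A new hit halts the target's ComboRunner and adds PushForce along the hit normal to its velocity, twice as wired.
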(event EventBeginPlay
  (Variables|Default|SetMesh (Actor|GetComponentbyClass (Components|GetOwner) "/Script/Engine.SkeletalMeshComponent")))

(event EventTick
  (params (DeltaSeconds :type Float%20%28single-precision%29))
  (if (Variables|Default|GetCasting)
    (CallFunction|HitCast)
    (else
      (Utilities|Set|Clear (Variables|Default|GetHitActors)))))

(fn HitCast
  (bind _mesh (Variables|Default|GetMesh))
  (bind (_outhits _returnvalue) (Class|KismetSystemLibrary|BoxTraceMultiforObjects (Transformation|GetSocketLocation _mesh "FX_weapon_tip") (Transformation|GetSocketLocation _mesh "FX_weapon_base") "64.000000,0.000000,64.000000" "0, 0, 0" (Utilities|Array|MakeArray "ObjectTypeQuery3") false 0 "None" true "(R=1.000000,G=0.000000,B=0.000000,A=1.000000)" "(R=0.000000,G=1.000000,B=0.000000,A=1.000000)" 0.5))
  (if _returnvalue
    (for _array_element _outhits
      (bind _new_actor (CallFunction|CheckNewActor _array_element))
      (if _new_actor
        (Utilities|FlowControl|Sequence
          (:then_0
            (CallFunction|TryHaltCombo _array_element))
          (:then_1
            _))
        (CallFunction|TryPushBack _array_element)))))

(fn EnableCast
  (Variables|Default|SetCasting true))

(fn DisableCast
  (Variables|Default|SetCasting false))

(fn TryHaltCombo
  (params (HitResult :type Hit%20Result%20Structure))
  (bind _returnvalue (Actor|GetComponentbyClass (.hitactor HitResult) "/Script/UE_AtherTest.ComboRunner"))
  (Utilities|IsValid _returnvalue
    (:Is%20Valid
      (Class|ComboRunner|HaltCombo _returnvalue))))

(fn TryPushBack
  (params (HitResult :type Hit%20Result%20Structure))
  (bind _returnvalue (Actor|GetComponentbyClass (.hitactor HitResult) "/Script/Engine.MovementComponent"))
  (Variables|/Script/Engine.MovementComponent|SetVelocity _returnvalue (+ (* (.normal HitResult) (Variables|Default|GetPushForce)) (Variables|/Script/Engine.MovementComponent|GetVelocity _returnvalue))))

(fn CheckNewActor
  (params (HitResult :type Hit%20Result%20Structure))
  (bind _hitactors (Variables|Default|GetHitActors))
  (if (Utilities|Set|Contains _hitactors (.hitactor HitResult))
    (return false)
    (else
      (Utilities|Set|Add _hitactors (.hitactor HitResult))
      (return true))))
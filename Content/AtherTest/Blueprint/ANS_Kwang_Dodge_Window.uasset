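; Anim notify state for Kwang's dodge window that warns nearby enemy AI of the owner's current combo action.
; It caches the current node name from the owner's ComboRunner component when its stored name is empty.
; Each tick it sphere-traces the Pawn profile around the owner, with debug drawing.
; For hits on actors tagged Enemy, it writes that name to their AI blackboard's ComingComboAction key.
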(fn GatherAroundEnemies
  (params (Caster :type Actor%20Object%20Reference))
  (bind _returnvalue (Transformation|GetActorLocation Caster))
  (bind (_outhits _returnvalue_2) (Class|KismetSystemLibrary|SphereTraceMultibyProfile Caster _returnvalue _returnvalue (Variables|Default|GetNotifyRadius) "Pawn" false 0 "ForOneFrame" true))
  (return _outhits _returnvalue_2))

(fn BroadcastComboAction
  (params (ComboName :type String) (HitResult :type Hit%20Result%20Structure))
  (if (Actor|ActorHasTag (.hitactor HitResult) "Enemy")
    (Class|BlackboardComponent|SetValueasString (AI|GetBlackboard (AI|GetAIController (.hitactor HitResult))) (Utilities|Name|MakeLiteralName "ComingComboAction") ComboName)
    (return)
    (else
      (return))))

(fn ReceivedNotifyTick
  (params (MeshComp :type Skeletal%20Mesh%20Component%20Object%20Reference) (Animation :type Anim%20Sequence%20Base%20Object%20Reference) (FrameDeltaTime :type Float%20%28single-precision%29) (EventReference :type Anim%20Notify%20Event%20Reference%20Structure%20%28by%20ref%29))
  (Utilities|FlowControl|Sequence
    (:then_0
      (if (Utilities|Array|IsEmpty (LocalVariables|GetComboActionName))
        (bind _returnvalue (Class|ComboRunner|GetCurrentNodeName (Actor|GetComponentbyClass (Components|GetOwner MeshComp) "/Script/UE_AtherTest.ComboRunner")))
        (LocalVariables|SetComboActionName _returnvalue)))
    (:then_1
      (bind (_outhits _returnvalue_2) (CallFunction|GatherAroundEnemies (Components|GetOwner MeshComp)))
      (if _returnvalue_2
        (for _array_element _outhits
          (CallFunction|BroadcastComboAction (LocalVariables|GetComboActionName) _array_element)))
      (return false))))
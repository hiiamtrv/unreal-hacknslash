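; Enemy AI controller that runs the BT_AICharacter behavior tree on BeginPlay and reacts to perceived actors.
; Perception updates store the actor and stimulus, then call hearing and sight wrappers that pass them to HandlePlayerHearing and HandlePlayerSight with a player key name.
; GetWorldWaypoints calls UseBlackboard on BB_AICharacter and returns the waypoints of the BP_WaypointContainer stored under its WaypointContainer key.
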(event OnTargetPerceptionUpdated(AIPerception)
  (params (Actor :type Actor%20Object%20Reference) (Stimulus :type AI%20Stimulus%20Structure))
  (Variables|Default|SetStimulus Stimulus)
  (Variables|Default|SetActor Actor)
  (CallFunction|BPHandlePlayerHearing)
  (CallFunction|BPHandlePlayerSight))

(event EventBeginPlay
  (AI|RunBehaviorTree "/Game/AtherTest/Blueprint/BT_AICharacter.BT_AICharacter"))

(fn ConstructionScript)

(fn GetWorldWaypoints
  (bind _blackboardcomponent (Class|AIController|UseBlackboard "/Game/AtherTest/Blueprint/BB_AICharacter.BB_AICharacter"))
  (bind _asbp_waypoint_container (Utilities|Casting|CastToBP_WaypointContainer (AI|Components|Blackboard|GetValueasObject _blackboardcomponent (Utilities|Name|MakeLiteralName "WaypointContainer")))
    (:then
      (return (Variables|/Game/AtherTest/Blueprint/BP_WaypointContainer.BP_WaypointContainer_C|GetWaypoints _asbp_waypoint_container)))
    (:CastFailed
      (return 0))))

(fn BPHandlePlayerSight
  (Class|EnemyAIController|HandlePlayerSight (Variables|Default|GetActor) (Variables|Default|GetStimulus) (Utilities|"Player"String)))

(fn BPHandlePlayerHearing
  (Class|EnemyAIController|HandlePlayerHearing (Variables|Default|GetActor) (Variables|Default|GetStimulus) (Utilities|"Player"String)))
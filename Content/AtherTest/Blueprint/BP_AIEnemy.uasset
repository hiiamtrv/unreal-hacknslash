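; BP_AIEnemy is an AI enemy that tells its Kwang animation Blueprint when it is engaging a target player.
; Each Tick, it reads TargetPlayer from the AI controller's Blackboard and sets Engaging on ABP_Kwang when that target is within EngageDistance of its owner.
; It then resets its rotation to yaw only, teleporting physics, to stay upright.
; Helper functions wrap the Blackboard, target and anim instance lookups.
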(event EventTick
  (params (DeltaSeconds :type Float%20%28single-precision%29))
  (Utilities|FlowControl|Sequence
    (:then_0
      ;[1 1 1] Comment
      (bind (_actor _success) (CallFunction|GetBBTargetPlayer))
      (bind _asabp_kwang (CallFunction|GetKwang))
      (Variables|/Game/AtherTest/Animations/ABP_Kwang.ABP_Kwang_C|SetEngaging _asabp_kwang (and _success (<= (Transformation|GetDistanceTo (Components|GetOwner) _actor) (Variables|AI|GetEngageDistance)))))
    (:then_1
      ;[1 1 1] Comment
      (Transformation|SetActorRotation (Math|Rotator|MakeRotator 0.0 0.0 (.yaw (Transformation|GetActorRotation))) true))))

(fn ConstructionScript)

(fn GetAIBlackboard
  (return (Variables|/Script/AIModule.AIController|GetBlackboard (AI|GetAIController (Components|GetOwner)))))

(fn GetKwang
  (bind _asabp_kwang (Utilities|Casting|CastToABP_Kwang (Components|SkeletalMesh|GetAnimInstance (Actor|GetComponentbyClass "/Script/Engine.SkeletalMeshComponent")))
    (:then
      _)
    (:CastFailed
      _))
  (return _asabp_kwang))

(fn GETBBTargetPlayer
  (bind _blackboard (CallFunction|GetAIBlackboard))
  (bind _asactor (Utilities|Casting|CastToActor (AI|Components|Blackboard|GetValueasObject _blackboard (Utilities|Name|MakeLiteralName "TargetPlayer")))
    (:then
      (return _asactor true))
    (:CastFailed
      (return 0 false))))